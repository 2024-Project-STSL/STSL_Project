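; Player camera pawn for a card game that pans and zooms over the board and routes mouse interaction to cards.
; Cursor traces classify hits as Floor, Card or None, resolving cards through their CardStack, then send drag and hover messages.
; Keys or floor dragging pan the pawn, clamped each Tick to gamemode world borders.
; Zoom, active only during a drag, changes spring-arm length and rescales move speed.
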(event `self.ReceiveBeginPlay`
  (bind _asslgamemode (cast `/Game/Blueprint/SLGamemode` (`GameplayStatics.GetGameMode`)))
  (set `self.WorldBorder` (`SLGameModeBase.GetWorldBorder` _asslgamemode false)))

(event `self.ReceiveTick`
  (params (DeltaSeconds :type "Float (single-precision)"))
  (`|ExecutionSequence`
    (:`then_0`
      (`self.Handle Mouse`))
    (:`then_1`
      (`self.ClampToBorder`))))

(event `InputAxis|MoveCameraRight` :consume false
  (params (AxisValue :type "Float (single-precision)"))
  ;[1 1 1] 카메라 이동 (키보드)
  (if (not (`|EnumEquality` (`self.GetMouseDraggingType`) "Floor"))
    (`self.AddMovementInput` (`KismetMathLibrary.Vector_Right`) (* AxisValue (`self.MoveSpeed`)))))

(event `InputAxis|MoveCameraUp`
  (params (AxisValue :type "Float (single-precision)"))
  ;[1 1 1] 카메라 이동 (키보드)
  (if (not (`|EnumEquality` (`self.GetMouseDraggingType`) "Floor"))
    (`self.AddMovementInput` (`KismetMathLibrary.Vector_Forward`) (* AxisValue (`self.MoveSpeed`)))))

(event `Key|LeftMouseButton`
  (params (Key :type "Key Structure"))
  (bind _returnvalue (`self.GetMouseDraggingActor`))
  ;[1 1 1] 마우스 입력 처리
  (:`Pressed`
    (bind (_mousehittype _actoronmouse) (`self.GetMouseHitObject`))
    (`self.SetMouseDraggingType` _mousehittype)
    (`self.SetMouseDraggingActor` _actoronmouse)
    (message `MouseInputInterface.StartDrag` _actoronmouse))
  (:`Released`
    (`self.SetMouseDraggingType` "None")
    (if (`KismetSystemLibrary.IsValid` _returnvalue)
      (message `MouseInputInterface.EndDrag` _returnvalue))))

(event `Handle Mouse`
  (bind _returnvalue (`self.GetMouseDraggingActor`))
  (bind _returnvalue_2 (`self.GetMouseHoveringActor`))
  (bind _returnvalue_3 (`self.GetMouseDraggingType`))
  ;[1 1 1] 마우스 입력 처리
  (`|ExecutionSequence`
    (:`then_0`
      (switch `EMouseHitObject` _returnvalue_3
        (:`Floor`
          (bind _returnvalue_4 (`WidgetLayoutLibrary.GetMousePositionOnPlatform`))
          (bind _returnvalue_5 (`self.GetMouseMovement` _returnvalue_4))
          (`self.AddMovementInput` _returnvalue_5 (* (`self.MoveSpeed`) 0.04))
          (set `self.MousePos` _returnvalue_4))
        (:`Card`
          (if (`KismetSystemLibrary.IsValid` _returnvalue)
            (message `MouseInputInterface.MoveToCursor` _returnvalue)))))
    (:`then_1`
      (if (`|EnumEquality` _returnvalue_3)
        (bind (_mousehittype _actoronmouse) (`self.GetMouseHitObject`))
        (if (not (== _actoronmouse _returnvalue_2))
          (if (`KismetSystemLibrary.IsValid` _returnvalue_2)
            (message `MouseInputInterface.EndMouseHover` _returnvalue_2))
          (`self.SetMouseHoveringActor` _actoronmouse)
          (message `MouseInputInterface.StartMouseHover` (`self.GetMouseHoveringActor`)))))))

(event `InputAxis|ZoomCamera`
  (params (AxisValue :type "Float (single-precision)"))
  (bind _springarm (`self.SpringArm`))
  ;[1 1 1] 줌인, 줌아웃
  (if (not (`|EnumEquality` (`self.GetMouseDraggingType`)))
    (bind _output_get (set `SpringArmComponent.TargetArmLength` (`KismetMathLibrary.FClamp` (+ (`SpringArmComponent.TargetArmLength` _springarm) (* AxisValue (`self.ZoomSpeed`))) (`self.SpringArmLengthMin`) (`self.SpringArmLengthMax`)) _springarm))
    (set `self.MoveSpeed` (* _output_get 0.0001))))

(event `ClampToBorder`
  (bind _worldborder (`self.WorldBorder`))
  ;[1 1 1] 이동 영역 제한
  (`self.K2_SetActorLocation` (`KismetMathLibrary.MakeVector` (`KismetMathLibrary.FClamp` (.x (`self.K2_GetActorLocation`)) (`BlueprintMapLibrary.Map_Find` _worldborder "Down") (`BlueprintMapLibrary.Map_Find` _worldborder "Up")) (`KismetMathLibrary.FClamp` (.y (`self.K2_GetActorLocation`)) (`BlueprintMapLibrary.Map_Find` _worldborder "Left") (`BlueprintMapLibrary.Map_Find` _worldborder "Right")) (.z (`self.K2_GetActorLocation`))) false true))

(fn `GetLastDraggingCard`
  (returns (Card :type "Actor Object Reference"))
  (bind _asslgamemode (cast `/Game/Blueprint/SLGamemode` (`GameplayStatics.GetGameMode`)))
  (return (`CardStack.GetLastCard` (`SLGameModeBase.GetDraggingStack` _asslgamemode))))

(fn `GetMouseHitObject`
  (returns (MouseHitType :type "EMouseHitObject Enum") (ActorOnMouse :type "Actor Object Reference"))
  (locals (MouseHit :type "EMouseHitObject Enum"))
  (bind (_bblockinghit _binitialoverlap _time _distance _location _impactpoint _normal _impactnormal _physmat _hitactor _hitcomponent) (`GameplayStatics.BreakHitResult` (`PlayerController.GetHitResultUnderCursorByChannel` (`GameplayStatics.GetPlayerController` 0) "TraceTypeQuery1" true)))
  (if (> (.z _location) 0.1)
    (bind _ascard (cast `Card` _hitactor)
      (:`then`
        (bind _output_get (set `local.MouseHit` "Card"))
        (bind _ascard_stack (cast `CardStack` (`Card.GetCardStack` _ascard)))
        (return _output_get (`CardStack.FindMouseSender` _ascard_stack _location)))
      (:`CastFailed`
        (set `local.MouseHit` "None")))
    (else
      (bind _output_get_2 (set `local.MouseHit` "Floor"))))
  (return _output_get_2 _hitactor))

(fn `GetMouseMovement`
  (params (CurrentMousePos :type "Vector2D Structure"))
  (returns (ReturnValue :type "Vector Structure"))
  (bind (_x _y) (`KismetMathLibrary.BreakVector2D` (- (`self.MousePos`) CurrentMousePos)))
  (return (`KismetMathLibrary.Conv_Vector2DToVector` (`KismetMathLibrary.MakeVector2D` (* _y -1.0) _x))))

(fn `UserConstructionScript`)