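; Card actor that the player can drag across the scene with the mouse cursor.
; StartDrag disables gravity on the Cube and stores the 2D offset between the card and the cursor's visibility trace hit.
; MovetoCursor teleports the card to the traced point plus that offset at FloatingHeight, and EndDrag restores gravity.
; These drag events are not called within this graph, and BeginPlay and Tick are empty.
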(event `self.ReceiveTick`
  (params (DeltaSeconds :type "Float (single-precision)")))

(event `self.ReceiveBeginPlay`)

(event `/Game/Blueprint/MouseInputInterface.Move to Cursor`
  (`self.K2_SetActorLocation` (`KismetMathLibrary.Conv_Vector2DToVector` (+ (`KismetMathLibrary.Conv_VectorToVector2D` (`.Location` (`GameplayStatics.BreakHitResult` (`PlayerController.GetHitResultUnderCursorByChannel` (`GameplayStatics.GetPlayerController` 0) "TraceTypeQuery1" true)))) (stale `/Game/Blueprint/MouseInputInterface.StartDrag` _output_get)) (`self.FloatingHeight`)) false true))

(event `/Game/Blueprint/MouseInputInterface.StartDrag`
  (`PrimitiveComponent.SetEnableGravity` (`self.Cube`) false)
  (bind _output_get (set `self.CardOffset` (`KismetMathLibrary.Conv_VectorToVector2D` (- (`self.K2_GetActorLocation`) (`.Location` (`GameplayStatics.BreakHitResult` (`PlayerController.GetHitResultUnderCursorByChannel` (`GameplayStatics.GetPlayerController` 0) "TraceTypeQuery1" true))))))))

(event `/Game/Blueprint/MouseInputInterface.EndDrag`
  (`PrimitiveComponent.SetEnableGravity` (`self.Cube`) true))

(fn `UserConstructionScript`)