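; SLGamemode is a game mode Blueprint that sets up a card-stack game when play begins.
; BeginPlay adds an AddCardButton widget to the viewport and calls SpawnCard for two starting cards at separate locations.
; The SpawnCardBP function spawns a CardStack and a Card at a given location, assigns the card ID, then adds the card to that stack.
; BeginPlay calls SpawnCard rather than SpawnCardBP, and SpawnCard is not defined in this graph.
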(event `self.ReceiveBeginPlay`
  (bind _returnvalue (`|GenericCreateObject` "/Game/Blueprint/AddCardButton.AddCardButton_C"))
  (`UserWidget.AddToViewport` _returnvalue 0)
  (`self.SpawnCard` (`KismetMathLibrary.MakeVector` 0.0) 3)
  (`self.SpawnCard` (`KismetMathLibrary.MakeVector` 500.0) 4))

(fn `SpawnCardBP`
  (params (Location :type "Vector Structure (by ref)") (CardID :type Integer))
  (bind _returnvalue (`KismetMathLibrary.Conv_VectorToTransform` Location))
  (bind _returnvalue_2 (`|SpawnActorFromClass` "/Script/STSL.CardStack" _returnvalue "Undefined" "MultiplyWithRoot" null null))
  (bind _returnvalue_3 (`|SpawnActorFromClass` "/Script/STSL.Card" _returnvalue "Undefined" "MultiplyWithRoot" null null))
  (`Card.SetCardID` _returnvalue_3 CardID)
  (`CardStack.AddCard` _returnvalue_2 _returnvalue_3))

(fn `UserConstructionScript`)